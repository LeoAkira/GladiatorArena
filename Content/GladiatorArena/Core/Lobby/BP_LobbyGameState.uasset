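; Lobby game state for Gladiator Arena that runs the room screen and starts the match when everyone is ready.
; It rebuilds the player list from PlayerArray on join or ready changes, enabling Ready only with two players.
; All-ready starts a countdown, using RetriggerableDelay and a cancellable Gate before the authority seamless-travels to Arena.
; Host-side list changes reset local ready status; Leave destroys the session and returns to MainMenu.
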(event Custom|OnReadyClicked
  (params (Status :type Boolean))
  (bind _asbp_lobby_player_state (Utilities|Casting|CastToBP_LobbyPlayerState (Variables|/Script/Engine.Controller|GetPlayerState (Game|GetPlayerController 0))))
  (Default|SetReadyStatus _asbp_lobby_player_state Status))

(event Custom|PlayerReadyChanged
  (CallFunction|SetupPlayerList)
  (CallFunction|CheckAllReady))

(event Custom|CheckAllReady
  (bind _lobbyroomscreen (Variables|Default|GetLobbyRoomScreen))
  (bind _countdowntime (Variables|Default|GetCountdownTime))
  (bind _ready (CallFunction|AreAllPlayersReady))
  (if _ready
    (Default|StartCountdown _lobbyroomscreen _countdowntime)
    (Utilities|FlowControl|Sequence
      (:then_0
        (Utilities|FlowControl|RetriggerableDelay _countdowntime)
        (Utilities|FlowControl|Gate true :!label _label
          (:Exit
            (Networking|SwitchHasAuthority
              (:Authority
                (Class|BaseGameMode|SeamlessTravel (Variables|Default|GetLobbyGameMode) "Arena"))))))
      (:then_1
        (goto _label Open)))
    (else
      (Default|StopCountdown _lobbyroomscreen)
      (goto _label Close))))

(event Custom|OnLeaveClicked
  (CallFunction|OnReadyClicked false)
  (|DestroySession (Game|GetPlayerController 0)
    (:OnSuccess
      (Game|OpenLevel(byName) "MainMenu"))))

(event Custom|PlayerListChanged
  (Utilities|FlowControl|Delay 0.2)
  (CallFunction|OnReadyClicked false)
  (CallFunction|SetupPlayerList))

(event EventBeginPlay
  (bind _returnvalue (Game|GetPlayerController 0))
  (Utilities|FlowControl|Sequence
    (:then_0
      (bind _returnvalue_2 (UserInterface|CreateWidget "/AssessmentAssets/UI/Lobby/WBP_LobbyRoom_Screen.WBP_LobbyRoom_Screen_C"))
      (bind _output_get (Variables|Default|SetLobbyRoomScreen _returnvalue_2))
      (UserInterface|Viewport|AddtoViewport _output_get 0)
      (Variables|/Script/Engine.PlayerController|SetbShowMouseCursor _returnvalue true)
      (Input|SetInputModeUIOnly _returnvalue _output_get "DoNotLock" false)
      (EventDispatchers|AssignOnReadyClicked _output_get (EventDispatchers|CreateEvent :!event Custom|OnReadyClicked))
      (EventDispatchers|BindEventtoOnLeaveClicked _output_get (EventDispatchers|CreateEvent :!event Custom|OnLeaveClicked)))
    (:then_1
      ;[1 1 1] TODO: Move to C++ PostInit
      (Utilities|FlowControl|Delay 0.2)
      (CallFunction|SetupPlayerList))
    (:then_2
      (Networking|SwitchHasAuthority
        (:Authority
          (bind _asbp_lobby_game_mode (Utilities|Casting|CastToBP_LobbyGameMode (Game|GetGameMode)))
          (bind _output_get_2 (Variables|Default|SetLobbyGameMode _asbp_lobby_game_mode))
          (EventDispatchers|BindEventtoOnPlayerListChanged _output_get_2 (delegate Custom|PlayerListChanged)))))))

(fn ConstructionScript)

(fn GetPlayers
  (return 0))

(fn SetupPlayerList
  (for _array_element (Variables|Default|GetPlayerArray)
    (bind _asbp_lobby_player_state (Utilities|Casting|CastToBP_LobbyPlayerState _array_element))
    (Utilities|Map|Add (LocalVariables|GetLocalList) (PlayerState|GetPlayerName _asbp_lobby_player_state) (Variables|/Game/GladiatorArena/Core/Lobby/BP_LobbyPlayerState.BP_LobbyPlayerState_C|GetbReady _asbp_lobby_player_state))
    (Math|Integer|IncrementInt (LocalVariables|GetCount)))
  (Default|UpdatePlayerList (Variables|Default|GetLobbyRoomScreen) (LocalVariables|GetLocalList))
  (Default|SetReadyButtonEnabled (Variables|Default|GetLobbyRoomScreen) (== (LocalVariables|GetCount) 2))
  (return))

(fn AreAllPlayersReady
  (for _array_element (Variables|Default|GetPlayerArray)
    (bind _asbp_lobby_player_state (Utilities|Casting|CastToBP_LobbyPlayerState _array_element))
    (if (not (Variables|/Game/GladiatorArena/Core/Lobby/BP_LobbyPlayerState.BP_LobbyPlayerState_C|GetbReady _asbp_lobby_player_state))
      (return false)))
  (return true))