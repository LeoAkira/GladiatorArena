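; Player controller for GladiatorArena that turns axis inputs into pawn movement and camera look.
; Move axes add movement input along the controlled pawn's forward and right vectors.
; Look axes add yaw and pitch input, then vertical look clamps the control rotation's pitch to a narrow symmetric range around level.
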(event EventBeginPlay)

(event EventTick
  (params (DeltaSeconds :type Float%20%28single-precision%29)))

(event Input|AxisEvents|InputAxisMoveForwardBackward
  (params (AxisValue :type Float%20%28single-precision%29))
  (bind _returnvalue (Pawn|GetControlledPawn))
  (Pawn|Input|AddMovementInput _returnvalue (Transformation|GetActorForwardVector _returnvalue) AxisValue false))

(event Input|AxisEvents|InputAxisMoveLeftRight
  (params (AxisValue :type Float%20%28single-precision%29))
  (bind _returnvalue (Pawn|GetControlledPawn))
  (Pawn|Input|AddMovementInput _returnvalue (Transformation|GetActorRightVector _returnvalue) AxisValue false))

(event Input|AxisEvents|InputAxisLookLeftRight
  (params (AxisValue :type Float%20%28single-precision%29))
  (Class|PlayerController|AddYawInput AxisValue))

(event Input|AxisEvents|InputAxisLookUpDown
  (params (AxisValue :type Float%20%28single-precision%29))
  (bind _returnvalue (Pawn|GetControlRotation :!class /Script/Engine.Controller))
  (bind _result (Math|Float|NegateFloat AxisValue)
    (:%20%20
      (Class|PlayerController|AddPitchInput _result)
      (Pawn|SetControlRotation (Math|Rotator|MakeRotator (.roll _returnvalue) (Math|Float|ClampAngle (.pitch _returnvalue) -3e+01 3e+01) (.yaw _returnvalue))))))

(fn ConstructionScript)