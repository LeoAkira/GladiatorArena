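; Player controller for the Gladiator Arena that controls player input, shows the end-game screen and handles leaving the match.
; It sets game-only input mode and disables input on BeginPlay, exposing ToggleInput to switch it on or off.
; AddEndGameScreen creates the end-game widget with the win result and countdown.
; Releasing the Exit action calls DestroySession and opens the MainMenu level from its immediate exec output.
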(event Custom|ToggleInput
  (params (Enabled :type Boolean))
  (bind _self self)
  (if Enabled
    (Input|EnableInput _self)
    (else
      (Input|DisableInput _self))))

(event Custom|AddEndGameScreen
  (params (bHasWon :type Boolean) (Countdown :type Float%20%28double-precision%29))
  (bind _returnvalue (UserInterface|CreateWidget "/AssessmentAssets/UI/EndGame/WBP_EndGame_Screen.WBP_EndGame_Screen_C" self Countdown bHasWon))
  (UserInterface|Viewport|AddtoViewport _returnvalue 0))

(event EventBeginPlay
  (Input|SetInputModeGameOnly self false)
  (CallFunction|ToggleInput false))

(event Input|ActionEvents|InputActionExit
  (params (Key :type Key%20Structure :default "None"))
  (:Released
    (|DestroySession self
      (:then
        (Game|OpenLevel(byName) "MainMenu")))))

(fn ConstructionScript)