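; Player character for GladiatorArena, handling movement, pitch-clamped camera look and Gameplay Ability System attacks, with abilities granted on BeginPlay.
; A gate-and-delay ClickOrHold macro turns Attack into normal (click) or heavy (hold) attack abilities.
; Tick derives yaw-relative velocity and Moving for animation and prints health; SetState sets walk speed from a map.
; Axe box overlap sends itself a Hit gameplay event only when the other actor is itself.
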(event OnComponentBeginOverlap(AxeDamageBox)
  (params (OverlappedComponent :type Primitive%20Component%20Object%20Reference) (OtherActor :type Actor%20Object%20Reference) (OtherComp :type Primitive%20Component%20Object%20Reference) (OtherBodyIndex :type Integer) (bFromSweep :type Boolean) (SweepResult :type Hit%20Result%20Structure%20%28by%20ref%29))
  (bind _self self)
  (if (not (!= OtherActor _self))
    (Ability|SendGameplayEventtoActor _self "(TagName=\"GameplayCue.Hit\")" (Utilities|Struct|MakeGameplayEventData "(TagName=\"GameplayCue.Hit\")" _self))))

(event EventBeginPlay
  (CallFunction|SetState "NewEnumerator0")
  (for _array_element (Variables|Default|GetAbilities)
    (GameplayAbilities|GiveAbility (Variables|Default|GetAbilitySystemComponent) _array_element 0 -1)))

(event Collision|EventActorBeginOverlap
  (params (OtherActor :type Actor%20Object%20Reference)))

(event EventTick
  (params (DeltaSeconds :type Float%20%28single-precision%29))
  (CallFunction|UpdateAnimationValues)
  (Development|PrintString (Utilities|String|ToString(Float) (.CurrentValue (Utilities|Struct|BreakGameplayAttributeData (Variables|/Script/GladiatorArena.BaseAttributeSet|GetHealth (Variables|Default|GetBaseAttributeSet))))) true true "(R=0.000000,G=0.660000,B=1.000000,A=1.000000)" DeltaSeconds))

(event Input|ActionEvents|InputActionAttack
  (params (Key :type Key%20Structure :default "None"))
  (bind _abilitysystemcomponent (Variables|Default|GetAbilitySystemComponent))
  ;[1 1 1] Player Input
  (:Pressed
    (Utilities|ClickorHold 0.4 :!label _label
      (:Click
        (Abilities|TryActivateAbilitybyClass _abilitysystemcomponent "/Game/GladiatorArena/Character/GameplayAbilities/BP_GA_Attack.BP_GA_Attack_C" true))
      (:Hold
        (Abilities|TryActivateAbilitybyClass _abilitysystemcomponent "/Game/GladiatorArena/Character/GameplayAbilities/BP_GA_HeavyAttack.BP_GA_HeavyAttack_C" true))))
  (:Released
    (goto _label Released)))

(event Input|ActionEvents|InputActionBlock
  (params (Key :type Key%20Structure :default "None"))
  ;[1 1 1] Player Input
)

(event Input|AxisEvents|InputAxisMoveForwardBackward
  (params (AxisValue :type Float%20%28single-precision%29))
  ;[1 1 1] Player Input
  (Pawn|Input|AddMovementInput (Transformation|GetActorForwardVector) AxisValue false))

(event Input|AxisEvents|InputAxisMoveLeftRight
  (params (AxisValue :type Float%20%28single-precision%29))
  ;[1 1 1] Player Input
  (Pawn|Input|AddMovementInput (Transformation|GetActorRightVector) AxisValue false))

(event Input|AxisEvents|InputAxisLookLeftRight
  (params (AxisValue :type Float%20%28single-precision%29))
  ;[1 1 1] Player Input
  (Pawn|Input|AddControllerYawInput AxisValue))

(event Input|AxisEvents|InputAxisLookUpDown
  (params (AxisValue :type Float%20%28single-precision%29))
  (bind _returnvalue (Pawn|GetControlRotation :!class /Script/Engine.Pawn))
  ;[1 1 1] Player Input
  (bind _result (Math|Float|NegateFloat AxisValue)
    (:%20%20
      (Pawn|Input|AddControllerPitchInput _result)
      (Pawn|SetControlRotation (Pawn|GetController) (Math|Rotator|MakeRotator (.roll _returnvalue) (Math|Float|ClampAngle (.pitch _returnvalue) -3e+01 3e+01) (.yaw _returnvalue))))))

(fn ConstructionScript)

(fn UpdateAnimationValues
  (bind _returnvalue (Transformation|GetActorRotation))
  (bind _charactermovement (Variables|Character|GetCharacterMovement))
  (bind _returnvalue_2 (Class|MovementComponent|GetMaxSpeed _charactermovement))
  (bind _yaw (Math|Rotator|BreakRotator _returnvalue))
  (bind _velocity (Variables|/Script/Engine.MovementComponent|GetVelocity _charactermovement))
  (bind _returnvalue_3 (/ _velocity _returnvalue_2))
  (bind _returnvalue_4 (Math|Vector|RotateVectorAroundAxis _returnvalue_3 _yaw "0.000000,0.000000,-1.000000"))
  (bind _returnvalue_5 (Math|Vector|VectorIsNearlyZero _returnvalue_4))
  (Utilities|FlowControl|Sequence
    (:then_0
      (if (!= (Math|Vector|VectorIsNearlyZero (Variables|Animation|GetScalarVelocity)) _returnvalue_5)
        (Variables|Animation|SetbMoving (not _returnvalue_5))))
    (:then_1
      (Variables|Animation|SetScalarVelocity _returnvalue_4)
      (return))))

(fn SetState
  (params (State :type States%20Enum :default "NewEnumerator0"))
  (bind _output_get (Variables|Default|SetState State))
  (Variables|/Script/Engine.CharacterMovementComponent|SetMaxWalkSpeed (Variables|Character|GetCharacterMovement) (.Value (Utilities|Map|Find (Variables|Default|GetStatesWalkSpeed) _output_get))))