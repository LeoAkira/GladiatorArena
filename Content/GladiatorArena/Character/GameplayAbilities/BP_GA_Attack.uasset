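; BP_GA_Attack is a Gladiator Arena gameplay ability that plays an attack montage and damages the player character it hits.
; It waits for a single GameplayCue.Hit event while the montage runs.
; The target's State selects either a shield or health damage effect, with magnitude passed through a SetByCaller tag, then triggers the target's OnHit.
; The ability ends when the montage completes, blends out, or is interrupted or cancelled.
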(event Ability|EventOnEndAbility
  (params (bWasCancelled :type Boolean))
  (|CallParentFunction bWasCancelled))

(event EventExecuteAbility
  (|CallParentFunction)
  (|PlayMontageandWaitProxy "None" (Variables|Default|GetMontage%20to%20Play) 1.0 "None" true 1.0 0.0 false
    (:then
      (bind _payload (Ability|Tasks|WaitGameplayEvent "(TagName=\"GameplayCue.Hit\")" 0 true)
        (:EventReceived
          (bind _asbp_player_character (Utilities|Casting|CastToBP_PlayerCharacter (.Target (Utilities|Struct|BreakGameplayEventData _payload))))
          (Variables|Default|SetTarget _asbp_player_character)
          (if (Utilities|Enum|Equal(Enum) (Variables|/Game/GladiatorArena/Character/BP_PlayerCharacter.BP_PlayerCharacter_C|GetState _asbp_player_character) "NewEnumerator2")
            (bind _returnvalue (Ability|GameplayEffect|AssignTagSetbyCallerMagnitude (Ability|MakeOutgoingGameplayEffectSpec "/Game/GladiatorArena/Character/GameplayEffects/BP_GE_DamageShield.BP_GE_DamageShield_C") "(TagName=\"SetByCaller.Damage\")" (Variables|Default|GetShieldDamage)))
            (GameplayEffects|ApplyGameplayEffectSpecToTarget (Ability|GetAbilitySystemComponent (.Instigator (Utilities|Struct|BreakGameplayEventData _payload))) _returnvalue (Ability|GetAbilitySystemComponent (.Target (Utilities|Struct|BreakGameplayEventData _payload))))
            (CallFunction|OnAttackHit)
            (else
              (bind _returnvalue_2 (Ability|GameplayEffect|AssignTagSetbyCallerMagnitude (Ability|MakeOutgoingGameplayEffectSpec "/Game/GladiatorArena/Character/GameplayEffects/BP_GE_DamageHealth.BP_GE_DamageHealth_C") "(TagName=\"SetByCaller.Damage\")" (Variables|Default|GetHealthDamage)))
              (GameplayEffects|ApplyGameplayEffectSpecToTarget (Ability|GetAbilitySystemComponent (.Instigator (Utilities|Struct|BreakGameplayEventData _payload))) _returnvalue_2 (Ability|GetAbilitySystemComponent (.Target (Utilities|Struct|BreakGameplayEventData _payload))))
              (CallFunction|OnAttackHit))))))
    (:OnCompleted
      (Ability|EndAbility :!label _label))
    (:OnBlendOut
      (goto _label))
    (:OnInterrupted
      (goto _label))
    (:OnCancelled
      (goto _label))))

(fn OnAttackHit
  (Default|OnHit (Variables|Default|GetTarget)))