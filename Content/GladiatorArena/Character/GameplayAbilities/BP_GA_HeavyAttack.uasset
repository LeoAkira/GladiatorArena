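; BP_GA_HeavyAttack is the Gladiator Arena heavy attack Gameplay Ability, which adds a stun to the hits it lands.
; Activation, execution and end events only forward to the parent ability, which supplies the base attack flow.
; On hit, it runs the parent handling, then uses the avatar's Ability System Component to apply BP_GE_Stun to the target's component.
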(event Ability|EventActivateAbility
  (|CallParentFunction))

(event Ability|EventOnEndAbility
  (params (bWasCancelled :type Boolean))
  (|CallParentFunction bWasCancelled))

(event EventOnAttackHit
  (|CallParentFunction)
  (GameplayEffects|ApplyGameplayEffectSpecToTarget (Ability|GetAbilitySystemComponent (Ability|GetAvatarActorfromActorInfo)) (Ability|MakeOutgoingGameplayEffectSpec "/Game/GladiatorArena/Character/GameplayEffects/BP_GE_Stun.BP_GE_Stun_C") (Ability|GetAbilitySystemComponent (Variables|Default|GetTarget))))

(event EventExecuteAbility
  (|CallParentFunction))