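; Base Gameplay Ability Blueprint for the player character that ties each ability to the character's state.
; On activation it stores the current state and proceeds only from the default state with a successful commit, otherwise cancelling.
; It then applies the ability's own state and calls ExecuteAbility, an empty hook for child abilities.
; On end, cancellation restores the stored state, while normal completion returns the character to the default state.
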(event Ability|EventActivateAbility
  (bind _asbp_player_character (Utilities|Casting|CastToBP_PlayerCharacter (Utilities|Struct|BreakGameplayAbilityActorInfo (Ability|GetActorInfo))))
  (bind _output_get (Variables|Default|SetCharacter _asbp_player_character))
  (Variables|Default|SetPrevState (Variables|/Game/GladiatorArena/Character/BP_PlayerCharacter.BP_PlayerCharacter_C|GetState _output_get))
  (if (Utilities|Enum|Equal(Enum) (Variables|/Game/GladiatorArena/Character/BP_PlayerCharacter.BP_PlayerCharacter_C|GetState _output_get) "NewEnumerator0")
    (bind _returnvalue (Ability|CommitAbility))
    (if _returnvalue
      (Default|SetState (Variables|Default|GetCharacter) (Variables|Default|GetAbilityState))
      (CallFunction|ExecuteAbility)
      (else
        (Ability|CancelAbility :!label _label)))
    (else
      (goto _label))))

(event Ability|EventOnEndAbility
  (params (bWasCancelled :type Boolean))
  (bind _character (Variables|Default|GetCharacter))
  (if bWasCancelled
    (Default|SetState _character (Variables|Default|GetPrevState))
    (else
      (Default|SetState _character "NewEnumerator0"))))

(fn ExecuteAbility)